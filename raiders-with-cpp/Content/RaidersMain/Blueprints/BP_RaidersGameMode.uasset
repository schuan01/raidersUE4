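; Raiders game mode Blueprint whose event graph holds only disconnected legacy setup, labelled as predating C++; BeginPlay and SpawnCharacterOLD are empty.
; The unused logic creates local players for 1vs1 or four-player team matches, based on a game instance flag.
; It spawns and possesses raiders at random team-filtered starts, assigning team, color and a free follow camera.
; FilterPlayerStarts returns the player starts matching a given team.
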(event Custom|SpawnCharacterOLD
  (params (PlayerController :type Player%20Controller%20Object%20Reference) (Team%20Assignment :type EOLDTeam%20Enum :default "NewEnumerator0") (CharacterColor :type Texture%202D%20Object%20Reference))
  ;[1 1 1] SPAWN BEFORE CPP
)

(event EventBeginPlay)

(fn ConstructionScript)

(fn FilterPlayerStarts
  (params (AllStarts :type Array%20of%20BP%20Raider%20Player%20Start%20Object%20References) (TeamFilter :type EOLDTeam%20Enum :default "NewEnumerator0"))
  (for _array_element AllStarts
    (if (Utilities|Enum|Equal(Enum) TeamFilter (Variables|/Game/RaidersMain/Blueprints/BP_RaiderPlayerStart.BP_RaiderPlayerStart_C|GetTeamStart_0 _array_element))
      (Utilities|Array|Add (LocalVariables|GettempPlayerTeam) _array_element)))
  (return (LocalVariables|GettempPlayerTeam)))