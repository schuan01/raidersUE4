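; Follow-camera actor for RaidersMain, now mostly a leftover shell from before a C++ rewrite, as its comments indicate.
; The old join event marks it used and makes it the joining controller's view target, while Tick, StartFollow and SetCameraPosP2 do nothing.
; Disconnected nodes retain the former logic: interpolated following of one player or a two-player midpoint, with arm length clamped from player separation.
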(event Custom|UpdateCameraOLD
  (CallFunction|StartFollow))

(event Custom|NewPlayerJoinOLD
  (params (NewPlayerController :type Player%20Controller%20Object%20Reference) (PlayerSpawn :type BP%20Raider%20Main%20Player%20Object%20Reference))
  (Variables|Default|SetisUsed true)
  (Game|Player|SetViewTargetwithBlend NewPlayerController self 0.0 "VTBlend_Linear" 0.0 false))

(event EventTick
  (params (DeltaSeconds :type Float%20%28single-precision%29))
  ;[1 1 1] BEFORE CPP
)

(fn ConstructionScript)

(fn SetCameraPosP2)

(fn StartFollow)