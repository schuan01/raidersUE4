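; BP_LootGeneric is a loot pickup that adds a resource to the raider player's inventory on overlap.
; BeginPlay builds a loot struct from its resource value, using its own class as the resource type.
; If the player can pick up, is below max level and still lacks required loot, it adds the struct, plays a sound, updates inventory UI and destroys itself.
; When that pickup completes the requirement, it flags and triggers the player's level-up readiness.
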(event OnComponentBeginOverlap(StaticMeshComponent)
  (params (OverlappedComponent :type Primitive%20Component%20Object%20Reference) (OtherActor :type Actor%20Object%20Reference) (OtherComp :type Primitive%20Component%20Object%20Reference) (OtherBodyIndex :type Integer) (bFromSweep :type Boolean) (SweepResult :type Hit%20Result%20Structure%20%28by%20ref%29))
  (bind _asbp_raider_main_player (Utilities|Casting|CastToBP_RaiderMainPlayer OtherActor))
  (if (Variables|/Game/RaidersMain/Blueprints/BP_RaiderMainPlayer.BP_RaiderMainPlayer_C|GetcanPickUpLoot _asbp_raider_main_player)
    (if (!= (Variables|/Game/RaidersMain/Blueprints/BP_RaiderMainPlayer.BP_RaiderMainPlayer_C|GetcurrentLVL _asbp_raider_main_player) 3)
      (bind _required (Default|HasLootRequired _asbp_raider_main_player (Variables|/Game/RaidersMain/Blueprints/BP_RaiderMainPlayer.BP_RaiderMainPlayer_C|GetcurrentLVL _asbp_raider_main_player) (Variables|/Game/RaidersMain/Blueprints/BP_RaiderMainPlayer.BP_RaiderMainPlayer_C|GetlistLootStructures _asbp_raider_main_player)))
      (if (not _required)
        (Utilities|Array|Add (Variables|/Game/RaidersMain/Blueprints/BP_RaiderMainPlayer.BP_RaiderMainPlayer_C|GetlistLootStructures _asbp_raider_main_player) (Variables|Default|GetlootStructure))
        (Audio|PlaySoundatLocation "/Game/RaidersMain/Sounds/Resource_Pick.Resource_Pick" (Transformation|GetWorldLocation (Variables|Default|GetStaticMeshComponent)) "0, 0, 0" 1.0 1.0 0.0 "/Game/RaidersMain/Sounds/FX_Attenuation.FX_Attenuation" 0 0)
        (Default|UpdateUIInventory _asbp_raider_main_player)
        (bind _required_2 (Default|HasLootRequired _asbp_raider_main_player (Variables|/Game/RaidersMain/Blueprints/BP_RaiderMainPlayer.BP_RaiderMainPlayer_C|GetcurrentLVL _asbp_raider_main_player) (Variables|/Game/RaidersMain/Blueprints/BP_RaiderMainPlayer.BP_RaiderMainPlayer_C|GetlistLootStructures _asbp_raider_main_player)))
        (if _required_2
          (Variables|/Game/RaidersMain/Blueprints/BP_RaiderMainPlayer.BP_RaiderMainPlayer_C|SetcanLevelUp _asbp_raider_main_player true)
          (Default|ReachLevelUp _asbp_raider_main_player))
        (Actor|DestroyActor)))))

(event EventBeginPlay
  (Variables|Default|SetlootStructure (Utilities|Struct|MakeLootStructure (Variables|Default|GetresourceValue) (Utilities|GetClass self))))

(fn ConstructionScript)