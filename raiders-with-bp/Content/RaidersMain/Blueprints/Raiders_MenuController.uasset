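; Raiders_MenuController is a menu controller that forwards player button presses to the main menu widget.
; Action, Attack_1 and Attack_Special inputs trigger the widget's accept, action and back button functions, matching the bottom, left and right face buttons.
; Raw A, X and B key events share the same calls as those input actions, and only presses are handled.
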(event Input|ActionEvents|InputActionAction
  (params (Key :type Key%20Structure :default "None"))
  ;[1 1 1] BUTTON FACE BOTTOM
  (:Pressed
    (Default|UseAcceptButton (Variables|Default|GetMainMenuWidget))))

(event Input|ActionEvents|InputActionAttack_Special
  (params (Key :type Key%20Structure :default "None"))
  ;[1 1 1] BUTTON FACE RIGHT
  (:Pressed
    (Default|UseBackButton (Variables|Default|GetMainMenuWidget))))

(event Input|ActionEvents|InputActionAttack_1
  (params (Key :type Key%20Structure :default "None"))
  ;[1 1 1] BUTTON FACE LEFT
  (:Pressed
    (Default|UseActionButton (Variables|Default|GetMainMenuWidget))))

(event Input|KeyboardEvents|A
  (params (Key :type Key%20Structure :default "None"))
  ;[1 1 1] BUTTON FACE BOTTOM
  (:Pressed
    (Default|UseAcceptButton (Variables|Default|GetMainMenuWidget))))

(event Input|KeyboardEvents|B
  (params (Key :type Key%20Structure :default "None"))
  ;[1 1 1] BUTTON FACE RIGHT
  (:Pressed
    (Default|UseBackButton (Variables|Default|GetMainMenuWidget))))

(event Input|KeyboardEvents|X
  (params (Key :type Key%20Structure :default "None"))
  ;[1 1 1] BUTTON FACE LEFT
  (:Pressed
    (Default|UseActionButton (Variables|Default|GetMainMenuWidget))))

(fn ConstructionScript)