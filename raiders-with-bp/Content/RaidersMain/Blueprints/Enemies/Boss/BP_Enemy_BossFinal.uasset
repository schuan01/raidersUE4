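; Final boss enemy that damages the player with claw hits, summons mini crabs and drops an item on death.
; Claw overlaps send damage to the player; the weapon toggle switches only the first claw's overlaps.
; Falling to a life threshold triggers a one-time crab wave, stepping a rotating arm to spread spawn points.
; A looping timer plays boss audio, and death stops movement and attacks before a delayed drop and destroy.
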(event OnComponentBeginOverlap(clawCollision)
  (params (OverlappedComponent :type Primitive%20Component%20Object%20Reference) (OtherActor :type Actor%20Object%20Reference) (OtherComp :type Primitive%20Component%20Object%20Reference) (OtherBodyIndex :type Integer) (bFromSweep :type Boolean) (SweepResult :type Hit%20Result%20Structure%20%28by%20ref%29))
  ;[1 1 1] SEND DAMAGE TO TARGET
  (if (!= OtherActor self)
    (bind _asbp_raider_main_player (Utilities|Casting|CastToBP_RaiderMainPlayer OtherActor))
    (CallFunction|SendDamagetoTarget _asbp_raider_main_player 0.0 0.0 "NewEnumerator3")))

(event OnComponentBeginOverlap(clawCollision2)
  (params (OverlappedComponent :type Primitive%20Component%20Object%20Reference) (OtherActor :type Actor%20Object%20Reference) (OtherComp :type Primitive%20Component%20Object%20Reference) (OtherBodyIndex :type Integer) (bFromSweep :type Boolean) (SweepResult :type Hit%20Result%20Structure%20%28by%20ref%29))
  ;[1 1 1] SEND DAMAGE TO TARGET
  (if (!= OtherActor self)
    (bind _asbp_raider_main_player (Utilities|Casting|CastToBP_RaiderMainPlayer OtherActor))
    (CallFunction|SendDamagetoTarget _asbp_raider_main_player 0.0 0.0 "NewEnumerator3")))

(event Custom|DropBossItem
  ;[1 1 1] DROP BOSS ITEM
  (Game|SpawnActorfromClass "/Game/RaidersMain/Blueprints/Enemies/Boss/BP_BossDrop.BP_BossDrop_C" (Math|Transform|MakeTransform (+ (.location (Transformation|GetActorTransform self)) "0, 0,5.000000" "")) "Undefined" 0 0))

(event Custom|PlaySound
  (Audio|PlaySoundatLocation "/Game/RaidersMain/Sounds/Sound_Cue_Boss.Sound_Cue_Boss" (Transformation|GetWorldLocation (Variables|Character|GetMesh)) "0, 0, 0" 1.0 1.0 0.0 "/Game/RaidersMain/Sounds/FX_Attenuation.FX_Attenuation" 0 0))

(event Custom|CrabsSpawner
  (bind _spawnerarm (Variables|Default|GetspawnerArm))
  (bind _relativerotation (Variables|/Script/Engine.SceneComponent|GetRelativeRotation _spawnerarm))
  ;[1 1 1] CRABS SPAWNER
  (for _index (range 1 (Variables|Spawner|GetamountOfSpawns))
    (Transformation|SetRelativeRotation _spawnerarm (Math|Rotator|MakeRotator (.roll _relativerotation) (.pitch _relativerotation) (+ (.yaw _relativerotation) (Variables|Spawner|Getrotation))) false false)
    (Game|SpawnActorfromClass "/Game/RaidersMain/Blueprints/Enemies/Melee/BP_Enemy_MiniCrabFromBoss.BP_Enemy_MiniCrabFromBoss_C" (Transformation|GetWorldTransform (Variables|Default|GetspawnerLocation)) "Undefined" 0 0)))

(event EventBeginPlay
  (|CallParentFunction)
  (Variables|/Script/Engine.PrimitiveComponent|SetbGenerateOverlapEvents (Variables|Default|Getweapon_mesh) false)
  (Variables|/Script/Engine.PrimitiveComponent|SetbGenerateOverlapEvents (Variables|Default|GetclawCollision) false)
  (Variables|/Script/Engine.PrimitiveComponent|SetbGenerateOverlapEvents (Variables|Default|GetclawCollision2) false)
  (Utilities|Time|SetTimerbyFunctionName 0 "PlaySound" 8.0 true))

(event Collision|EventActorBeginOverlap
  (params (OtherActor :type Actor%20Object%20Reference))
  (|CallParentFunction OtherActor) ; This node is disabled and will not be called.\nDrag off pins to build functionality.
)

(event EventToggleWeaponCollision
  (params (isActive :type Boolean))
  ;[1 1 1] SEND DAMAGE TO TARGET
  (|CallParentFunction isActive)
  (Variables|/Script/Engine.PrimitiveComponent|SetbGenerateOverlapEvents (Variables|Default|GetclawCollision) isActive))

(event EventTick
  (params (DeltaSeconds :type Float%20%28single-precision%29))
  (|CallParentFunction DeltaSeconds) ; This node is disabled and will not be called.\nDrag off pins to build functionality.
)

(event EventTriggerDeath
  ;[1 1 1] TRIGGER DEATH
  (Variables|Default|SetbaseDamage 0.0)
  (Variables|Default|SetisAttacking_1 false)
  (Variables|/Game/AIBehaviorToolkit/Blueprints/BP_BehaviorComponent.BP_BehaviorComponent_C|SetIsAlive (Variables|Default|GetBehaviorComponent) false)
  (Pawn|Components|CharacterMovement|SetMovementMode (Variables|Character|GetCharacterMovement) "MOVE_None" 0)
  (CallFunction|ToggleWeaponCollision false)
  (Audio|PlaySoundatLocation "/Game/RaidersMain/Sounds/Boss_Death.Boss_Death" (Transformation|GetWorldLocation (Variables|Character|GetMesh)) "0, 0, 0" 1.0 1.0 0.0 "/Game/RaidersMain/Sounds/FX_Attenuation.FX_Attenuation" 0 0)
  (Utilities|FlowControl|Delay 2.0)
  (CallFunction|DropBossItem)
  (Audio|PlaySoundatLocation "/Game/RaidersMain/Sounds/Pinza_Drop__Free_.Pinza_Drop__Free_" (Transformation|GetWorldLocation (Variables|Character|GetMesh)) "0, 0, 0" 1.0 1.0 0.0 0 0 0)
  (Actor|DestroyActor))

(event EventRecieveBPDamage
  (|CallParentFunction)
  (if (<= (Variables|Default|GetbaseLife) (Variables|Spawner|GetLifeForSpawner))
    (Utilities|FlowControl|DoOnce false
      (:Completed
        (CallFunction|CrabsSpawner)))))

(fn ConstructionScript
  (|CallParentFunction))