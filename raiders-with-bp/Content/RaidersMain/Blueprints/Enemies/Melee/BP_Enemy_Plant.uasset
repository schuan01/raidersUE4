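; Plant enemy that attacks by spawning projectiles, built on a parent enemy class.
; The inherited weapon-collision toggle doubles as the fire trigger, spawning a projectile owned by the plant at its spawn point, while weapon mesh overlaps are disabled at start.
; BeginPlay also sets weighted bone, wood and stone loot odds, picks a random drop and starts a looping timer for positional plant sounds, with a separate sound on death.
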(event Custom|SpawnProjectile
  ;[1 1 1] Projectile
  (bind _returnvalue (Game|SpawnActorfromClass "/Game/RaidersMain/Blueprints/Enemies/Melee/Plant/BP_PlantProjectile.BP_PlantProjectile_C" (Transformation|GetWorldTransform (Variables|Default|GetspawnLocation)) "AlwaysSpawn" 0 0))
  (Variables|/Game/RaidersMain/Blueprints/Enemies/Melee/Plant/BP_PlantProjectile.BP_PlantProjectile_C|SetprojectileOwner _returnvalue self))

(event Custom|PlaySound
  ;[1 1 1] Play Random Sound
  (Audio|PlaySoundatLocation "/Game/RaidersMain/Sounds/Plant_FX.Plant_FX" (Transformation|GetWorldLocation (Variables|Character|GetMesh)) "0, 0, 0" 1.0 1.0 0.0 "/Game/RaidersMain/Sounds/FX_Attenuation.FX_Attenuation" 0 0))

(event EventBeginPlay
  ;[1 1 1] Begin Play
  (|CallParentFunction)
  (Variables|/Script/Engine.PrimitiveComponent|SetbGenerateOverlapEvents (Variables|Default|Getweapon_mesh) false)
  (Utilities|Time|SetTimerbyFunctionName 0 "PlaySound" 8.0 true)
  ;;[1 1 1] PROBABILITY
  (CallFunction|SetLootProbabilty 5 40 55)
  (CallFunction|ChooseRandomDropClass))

(event Collision|EventActorBeginOverlap
  (params (OtherActor :type Actor%20Object%20Reference))
  (|CallParentFunction OtherActor) ; This node is disabled and will not be called.\nDrag off pins to build functionality.
)

(event EventToggleWeaponCollision
  (params (isActive :type Boolean))
  ;[1 1 1] SEND DAMAGE TO TARGET
  (|CallParentFunction isActive)
  (if isActive
    (CallFunction|SpawnProjectile)))

(event EventTick
  (params (DeltaSeconds :type Float%20%28single-precision%29))
  (|CallParentFunction DeltaSeconds))

(event EventTriggerDeath
  ;[1 1 1] SEND DAMAGE TO TARGET
  (|CallParentFunction)
  (Audio|PlaySoundatLocation "/Game/RaidersMain/Sounds/Plant_Death.Plant_Death" (Transformation|GetWorldLocation (Variables|Character|GetMesh)) "0, 0, 0" 0.3 1.0 0.0 "/Game/RaidersMain/Sounds/FX_Attenuation.FX_Attenuation" 0 0))

(fn ConstructionScript
  (|CallParentFunction))