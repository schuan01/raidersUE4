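; Melee pirate enemy, built on a parent enemy class that supplies the damage, loot and death logic it calls.
; Weapon mesh overlaps are off at start, follow the parent's weapon-collision toggle, and send damage when they hit a player.
; On spawn it weights loot entirely to bone, picks a drop class and starts a looping timer for pirate voice sounds at a randomized interval.
; Death adds its own positional sound.
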(event OnComponentBeginOverlap(weapon_mesh)
  (params (OverlappedComponent :type Primitive%20Component%20Object%20Reference) (OtherActor :type Actor%20Object%20Reference) (OtherComp :type Primitive%20Component%20Object%20Reference) (OtherBodyIndex :type Integer) (bFromSweep :type Boolean) (SweepResult :type Hit%20Result%20Structure%20%28by%20ref%29))
  ;[1 1 1] SEND DAMAGE TO TARGET
  (if (!= OtherActor self)
    (bind _asbp_raider_main_player (Utilities|Casting|CastToBP_RaiderMainPlayer OtherActor))
    (CallFunction|SendDamagetoTarget _asbp_raider_main_player 0.0 0.0 "NewEnumerator3")))

(event Custom|PlaySound
  (Audio|PlaySoundatLocation "/Game/RaidersMain/Sounds/Sound_Cue_Pirate.Sound_Cue_Pirate" (Transformation|GetWorldLocation (Variables|Character|GetMesh)) "0, 0, 0" 1.0 1.0 0.0 "/Game/RaidersMain/Sounds/FX_Attenuation.FX_Attenuation" 0 0))

(event EventBeginPlay
  (|CallParentFunction)
  (Variables|/Script/Engine.PrimitiveComponent|SetbGenerateOverlapEvents (Variables|Default|Getweapon_mesh) false)
  (Utilities|Time|SetTimerbyFunctionName 0 "PlaySound" (Math|Random|RandomFloatinRange 1e+01 15.0) true)
  ;[1 1 1] PROBABILITY
  (CallFunction|SetLootProbabilty 100)
  (CallFunction|ChooseRandomDropClass))

(event Collision|EventActorBeginOverlap
  (params (OtherActor :type Actor%20Object%20Reference))
  (|CallParentFunction OtherActor) ; This node is disabled and will not be called.\nDrag off pins to build functionality.
)

(event EventToggleWeaponCollision
  (params (isActive :type Boolean))
  ;[1 1 1] SEND DAMAGE TO TARGET
  (|CallParentFunction isActive)
  (Variables|/Script/Engine.PrimitiveComponent|SetbGenerateOverlapEvents (Variables|Default|Getweapon_mesh) isActive))

(event EventTriggerDeath
  ;[1 1 1] Trigger Death
  (|CallParentFunction)
  (Audio|PlaySoundatLocation "/Game/RaidersMain/Sounds/Pirate_Death.Pirate_Death" (Transformation|GetWorldLocation (Variables|Character|GetMesh)) "0, 0, 0" 1.0 1.0 0.0 "/Game/RaidersMain/Sounds/FX_Attenuation.FX_Attenuation" 0 0))

(fn ConstructionScript
  (|CallParentFunction))