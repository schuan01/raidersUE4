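; BP_Enemy_MiniCrab is a melee crab enemy that damages the raider player with its claws.
; On BeginPlay it disables weapon and claw overlaps, starts a looping timer for its positional crab sound, and picks a random drop weighted toward stone.
; Claw overlaps send damage to BP_RaiderMainPlayer.
; ToggleWeaponCollision extends the parent to switch the first claw's overlaps, but always leaves the second claw's off.
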(event OnComponentBeginOverlap(clawCollision)
  (params (OverlappedComponent :type Primitive%20Component%20Object%20Reference) (OtherActor :type Actor%20Object%20Reference) (OtherComp :type Primitive%20Component%20Object%20Reference) (OtherBodyIndex :type Integer) (bFromSweep :type Boolean) (SweepResult :type Hit%20Result%20Structure%20%28by%20ref%29))
  ;[1 1 1] SEND DAMAGE TO TARGET
  (if (!= OtherActor self)
    (bind _asbp_raider_main_player (Utilities|Casting|CastToBP_RaiderMainPlayer OtherActor))
    (CallFunction|SendDamagetoTarget _asbp_raider_main_player 0.0 0.0 "NewEnumerator3")))

(event OnComponentBeginOverlap(clawCollision2)
  (params (OverlappedComponent :type Primitive%20Component%20Object%20Reference) (OtherActor :type Actor%20Object%20Reference) (OtherComp :type Primitive%20Component%20Object%20Reference) (OtherBodyIndex :type Integer) (bFromSweep :type Boolean) (SweepResult :type Hit%20Result%20Structure%20%28by%20ref%29))
  ;[1 1 1] SEND DAMAGE TO TARGET
  (if (!= OtherActor self)
    (bind _asbp_raider_main_player (Utilities|Casting|CastToBP_RaiderMainPlayer OtherActor))
    (CallFunction|SendDamagetoTarget _asbp_raider_main_player 0.0 0.0 "NewEnumerator3")))

(event Custom|PlaySound
  (Audio|PlaySoundatLocation "/Game/RaidersMain/Sounds/MiniCrab_FX.MiniCrab_FX" (Transformation|GetWorldLocation (Variables|Character|GetMesh)) "0, 0, 0" 1.0 1.0 0.0 "/Game/RaidersMain/Sounds/FX_Attenuation.FX_Attenuation" 0 0))

(event EventBeginPlay
  (|CallParentFunction)
  (Variables|/Script/Engine.PrimitiveComponent|SetbGenerateOverlapEvents (Variables|Default|Getweapon_mesh) false)
  (Variables|/Script/Engine.PrimitiveComponent|SetbGenerateOverlapEvents (Variables|Default|GetclawCollision) false)
  (Variables|/Script/Engine.PrimitiveComponent|SetbGenerateOverlapEvents (Variables|Default|GetclawCollision2) false)
  (Utilities|Time|SetTimerbyFunctionName 0 "PlaySound" 8.0 true)
  ;[1 1 1] PROBABILITY
  (CallFunction|SetLootProbabilty 5 25 70)
  (CallFunction|ChooseRandomDropClass))

(event Collision|EventActorBeginOverlap
  (params (OtherActor :type Actor%20Object%20Reference))
  (|CallParentFunction OtherActor) ; This node is disabled and will not be called.\nDrag off pins to build functionality.
)

(event EventToggleWeaponCollision
  (params (isActive :type Boolean))
  ;[1 1 1] SEND DAMAGE TO TARGET
  (|CallParentFunction isActive)
  (Variables|/Script/Engine.PrimitiveComponent|SetbGenerateOverlapEvents (Variables|Default|GetclawCollision) isActive)
  (Variables|/Script/Engine.PrimitiveComponent|SetbGenerateOverlapEvents (Variables|Default|GetclawCollision2) false))

(event EventTick
  (params (DeltaSeconds :type Float%20%28single-precision%29))
  (|CallParentFunction DeltaSeconds) ; This node is disabled and will not be called.\nDrag off pins to build functionality.
)

(fn ConstructionScript
  (|CallParentFunction))