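; BP_RaiderCharacter is a Raiders character Blueprint that handles weapon damage, hit feedback and death.
; ToggleWeaponCollision switches the weapon's overlap events, which start off, while SendDamageToTarget picks damage by attack type and applies it through the target's ReceiveDamage and DoFinalDamageToLife.
; Positive damage updates the victim controller's health UI and plays a hit or death sound; zero life triggers death, disabling capsule collision.
; RecieveBPDamage is an empty hook, and the construction script's weapon-socket attachment is disconnected.
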(event Custom|ToggleWeaponCollision
  (params (isActive :type Boolean))
  ;[1 1 1] TOGGLE WEAPON COLLISION
  (Variables|/Script/Engine.PrimitiveComponent|SetbGenerateOverlapEvents (Variables|Default|GetWeaponCollision) isActive))

(event Custom|SendDamageToTarget
  (params (CharacterDestination :type Raiders%20Base%20Character%20Object%20Reference) (BaseDamageAttack1 :type Float%20%28single-precision%29) (BaseDamageAttack2 :type Float%20%28single-precision%29) (AttackType :type EAttackType%20Enum :default "NewEnumerator3"))
  ;[1 1 1] SEND DAMAGE TO TARGET
  (Utilities|FlowControl|Sequence
    (:then_0
      (switch Utilities|FlowControl|Switch|SwitchonEAttackType AttackType
        (:NewEnumerator0
          (Variables|Default|SetcurrentDamage BaseDamageAttack1))
        (:NewEnumerator1
          (Variables|Default|SetcurrentDamage BaseDamageAttack2))
        (:NewEnumerator2
          (Variables|Default|SetcurrentDamage (Variables|Default|GetbaseDamage) :!label _label))
        (:NewEnumerator3
          (goto _label))))
    (:then_1
      (bind _asbp_raider_character (Utilities|Casting|CastToBP_RaiderCharacter CharacterDestination))
      (CallFunction|RecieveBPDamage _asbp_raider_character)
      (Variables|Default|SetbaseLifeBeforeDamage (Variables|/Script/RaidersUE4.RaidersBaseCharacter|GetbaseLife CharacterDestination))
      (bind _returnvalue (Class|RaidersBaseCharacter|ReceiveDamage CharacterDestination (Variables|Default|GetcurrentDamage) (Variables|Default|GetbaseCritic)))
      (Class|RaidersBaseCharacter|DoFinalDamagetoLife CharacterDestination _returnvalue)
      (if (> _returnvalue 0.0)
        (CallFunction|UpdateDamageUI CharacterDestination _returnvalue (Variables|Default|GetbaseLifeBeforeDamage)))
      (Variables|Default|SetbaseLifeBeforeDamage 0.0)
      (if (<= (Variables|/Script/RaidersUE4.RaidersBaseCharacter|GetbaseLife CharacterDestination) 0.0)
        (bind _asbp_raider_character_2 (Utilities|Casting|CastToBP_RaiderCharacter CharacterDestination))
        (CallFunction|TriggerDeath _asbp_raider_character_2)))))

(event Custom|PlayHurtDamageSound
  (params (Sound :type Sound%20Base%20Object%20Reference))
  ;[1 1 1] PLAY SOUND AT LOCATION
  (Audio|PlaySoundatLocation Sound (Transformation|GetWorldLocation (Variables|Character|GetMesh)) "0, 0, 0" 1.0 1.0 0.0 0 0 0))

(event Custom|TriggerDeath
  ;[1 1 1] TRIGGER DEATH
  (Variables|Default|SetisDead true)
  (Collision|SetCollisionEnabled (Variables|Default|GetCapsuleComponent) "NoCollision"))

(event Custom|UpdateDamageUI
  (params (Character :type Raiders%20Base%20Character%20Object%20Reference) (Damage :type Float%20%28single-precision%29) (BaseLifeBeforeDamage :type Float%20%28single-precision%29))
  ;[1 1 1] UPDATE DAMAGE UI
  (bind _asraiders_third_person_controller (Utilities|Casting|CastToRaiders_ThirdPersonController (Pawn|GetController Character)))
  (Default|ReceiveDamageUpdateUI _asraiders_third_person_controller Damage BaseLifeBeforeDamage)
  (if (<= (Variables|/Script/RaidersUE4.RaidersBaseCharacter|GetbaseLife Character) 0.0)
    (CallFunction|PlayHurtDamageSound "/Game/RaidersMain/Sounds/Player_Death.Player_Death")
    (else
      (CallFunction|PlayHurtDamageSound "/Game/RaidersMain/Sounds/Player_Hit__Damage_.Player_Hit__Damage_"))))

(event Custom|RecieveBPDamage
  ;[1 1 1] SEND DAMAGE TO TARGET
)

(event EventBeginPlay
  ;[1 1 1] BEGIN PLAY
  (Variables|/Script/Engine.PrimitiveComponent|SetbGenerateOverlapEvents (Variables|Default|GetWeaponCollision) false))

(fn ConstructionScript)