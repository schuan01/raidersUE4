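; BP_Altar is a team altar where raiders level up and where a match can be won.
; Box overlaps show or hide a Plane indicator based on whether players can level up.
; An other-team player carrying the boss drop triggers end game once; without it, the altar re-applies their class via ChooseClass.
; AltarLevelUp checks team and required loot, clears the loot, then levels the player with effects and sound.
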(event OnComponentBeginOverlap(Box)
  (params (OverlappedComponent :type Primitive%20Component%20Object%20Reference) (OtherActor :type Actor%20Object%20Reference) (OtherComp :type Primitive%20Component%20Object%20Reference) (OtherBodyIndex :type Integer) (bFromSweep :type Boolean) (SweepResult :type Hit%20Result%20Structure%20%28by%20ref%29))
  (bind _asbp_raider_main_player (Utilities|Casting|CastToBP_RaiderMainPlayer OtherActor))
  (if (Utilities|Enum|Equal(Enum) (Variables|/Game/RaidersMain/Blueprints/BP_RaiderMainPlayer.BP_RaiderMainPlayer_C|Getteam _asbp_raider_main_player) (Variables|Default|GetcurrentTeam))
    ;[1 1 1] SHOW LEVEL UP BUTTON
    (if (Variables|/Game/RaidersMain/Blueprints/BP_RaiderMainPlayer.BP_RaiderMainPlayer_C|GetcanLevelUp _asbp_raider_main_player) :!label _label
      (Rendering|SetVisibility (Variables|Default|GetPlane) true false))
    (elif (Variables|/Game/RaidersMain/Blueprints/BP_RaiderMainPlayer.BP_RaiderMainPlayer_C|GethasBossDrop _asbp_raider_main_player)
      ;[1 1 1] END GFAME
      (if (Variables|Default|GetcanWin)
        (if (Utilities|Enum|NotEqual(Enum) (Variables|/Game/RaidersMain/Blueprints/BP_RaiderMainPlayer.BP_RaiderMainPlayer_C|Getteam _asbp_raider_main_player) "NewEnumerator2")
          (Utilities|FlowControl|DoOnce false
            (:Completed
              (Variables|Default|SetcanWin false)
              (Variables|Default|SetteamWin (Variables|/Game/RaidersMain/Blueprints/BP_RaiderMainPlayer.BP_RaiderMainPlayer_C|Getteam _asbp_raider_main_player))
              (Default|CallTriggerEndGame)))))
      (else
        (Utilities|FlowControl|Sequence
          (:then_0
            (goto _label))
          (:then_1
            (Default|ChooseClass _asbp_raider_main_player (Variables|/Game/RaidersMain/Blueprints/BP_RaiderMainPlayer.BP_RaiderMainPlayer_C|Getclass _asbp_raider_main_player))))))))

(event OnComponentEndOverlap(Box)
  (params (OverlappedComponent :type Primitive%20Component%20Object%20Reference) (OtherActor :type Actor%20Object%20Reference) (OtherComp :type Primitive%20Component%20Object%20Reference) (OtherBodyIndex :type Integer))
  (Variables|Default|SettempCanLvlUp false)
  (for _array_element (Collision|GetOverlappingActors (Variables|Default|GetBox) "/Game/RaidersMain/Blueprints/BP_RaiderMainPlayer.BP_RaiderMainPlayer_C" :!class /Script/Engine.PrimitiveComponent)
    (bind _asbp_raider_main_player (Utilities|Casting|CastToBP_RaiderMainPlayer _array_element))
    (if (Variables|/Game/RaidersMain/Blueprints/BP_RaiderMainPlayer.BP_RaiderMainPlayer_C|GetcanLevelUp _asbp_raider_main_player)
      (Variables|Default|SettempCanLvlUp true)))
  (if (not (Variables|Default|GettempCanLvlUp))
    (Rendering|SetVisibility (Variables|Default|GetPlane) false false)))

(event Custom|AltarLevelUp
  (params (Player :type BP%20Raider%20Main%20Player%20Object%20Reference))
  (bind _rootcomponent (Variables|/Script/Engine.Actor|GetRootComponent Player))
  (bind _returnvalue (Transformation|GetWorldLocation _rootcomponent))
  ;[1 1 1] LEVEL UP
  (if (Utilities|Enum|Equal(Enum) (Variables|/Game/RaidersMain/Blueprints/BP_RaiderMainPlayer.BP_RaiderMainPlayer_C|Getteam Player) (Variables|Default|GetcurrentTeam))
    (bind _required (Default|HasLootRequired Player (Variables|/Game/RaidersMain/Blueprints/BP_RaiderMainPlayer.BP_RaiderMainPlayer_C|GetcurrentLVL Player) (Variables|/Game/RaidersMain/Blueprints/BP_RaiderMainPlayer.BP_RaiderMainPlayer_C|GetlistLootStructures Player)))
    (if _required
      (Utilities|FlowControl|DoOnce false :!label _label
        (:Completed
          ;;[1 1 1] REMOVE ALL CURRENT LOOT FROM PLAYER
          (Utilities|FlowControl|Sequence
            (:then_0
              (Default|RemoveAllLootStructs Player))
            (:then_1
              ;;[1 1 1] LEVEL UP
              (Default|LevelUpCharacter Player)
              (Effects|SpawnEmitteratLocation "/Game/InfinityBladeEffects/Effects/FX_Skill_Aura/P_Aura_Default_Upheaval_01.P_Aura_Default_Upheaval_01" _returnvalue)
              (Audio|PlaySoundatLocation "/Game/RaidersMain/Sounds/Player_LevelUp.Player_LevelUp" _returnvalue "0, 0, 0" 1.0 1.0 0.0 "/Game/RaidersMain/Sounds/FX_Attenuation.FX_Attenuation" 0 0)
              (Rendering|SetVisibility (Variables|Default|GetPlane) false false)
              (goto _label Reset))))))))

(fn ConstructionScript)