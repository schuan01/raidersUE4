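; Camera actor that becomes a joining player's view target and follows that player through the level.
; NewPlayerJoin marks the camera as used and stores the spawned player, then Tick calls StartFollow through UpdateCamera to ease the actor toward that player with VInterpTo.
; Shared two-player framing (midpoint position, distance-based spring arm length) remains in the graph but is disconnected, as is an old looping update timer.
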(event Custom|UpdateCamera
  (CallFunction|StartFollow))

(event Custom|NewPlayerJoin
  (params (NewPlayerController :type Player%20Controller%20Object%20Reference) (PlayerSpawn :type BP%20Raider%20Main%20Player%20Object%20Reference))
  (Variables|Default|SetisUsed true)
  (Game|Player|SetViewTargetwithBlend NewPlayerController self 0.0 "VTBlend_Linear" 0.0 false)
  (Variables|Default|SetPlayerToFollow PlayerSpawn))

(event EventBeginPlay)

(event EventTick
  (params (DeltaSeconds :type Float%20%28single-precision%29))
  (CallFunction|UpdateCamera))

(fn ConstructionScript)

(fn SetCameraPosP2
  (bind _asraiders_game_mode (Utilities|Casting|CastToRaidersGameMode (Game|GetGameMode)))
  (Variables|Default|SetTargetPos (/ (+ (Transformation|GetActorLocation (Variables|Default|GetP1)) (Transformation|GetActorLocation (Variables|Default|GetP2))) (Math|Conversions|ToFloat(Integer) (Utilities|Array|Length (Variables|/Game/RaidersMain/Blueprints/RaidersGameMode.RaidersGameMode_C|GetPlayers _asraiders_game_mode)))))
  (Transformation|SetActorLocation (Math|Interpolation|VInterpTo (Variables|Default|GetPreviousPos) (Variables|Default|GetTargetPos) (Utilities|Time|GetWorldDeltaSeconds) (Variables|Default|GetInterpSpeed)) false false)
  (Variables|Default|SetPreviousPos (Transformation|GetActorLocation)))

(fn StartFollow
  (bind _playertofollow (Variables|Default|GetPlayerToFollow)
    (:then
      (Variables|Default|SetTargetPos (Transformation|GetActorLocation _playertofollow))
      (Transformation|SetActorLocation (Math|Interpolation|VInterpTo (Variables|Default|GetPreviousPos) (Variables|Default|GetTargetPos) (Utilities|Time|GetWorldDeltaSeconds) (Variables|Default|GetInterpSpeed)) false false)
      (Variables|Default|SetPreviousPos (Transformation|GetActorLocation)))
    (:else)))