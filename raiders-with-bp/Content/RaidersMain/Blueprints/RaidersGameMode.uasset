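; Local multiplayer game mode that sets up Raiders matches as 1v1 or 2v2, based on the game instance flag.
; BeginPlay creates local player controllers, then SpawnCharacter swaps each existing pawn for a raider at a random team-filtered start, assigning team, color and a free follow camera.
; DespawnPlayer returns a controller to an InitPawn at any random start.
; Small events enable menu mode buttons and count detected inputs; legacy spawn logic remains unwired.
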(event Custom|Enable1VS1
  (Widget|SetIsEnabled (Variables|/Game/RaidersMain/UI/MainMenu.MainMenu_C|GetButton1VS1 (Variables|Default|GetWidgetMenu)) true))

(event Custom|Enable2VS2
  (Widget|SetIsEnabled (Variables|/Game/RaidersMain/UI/MainMenu.MainMenu_C|GetButton2VS2 (Variables|Default|GetWidgetMenu)) true))

(event Custom|AddInputDetected
  (Math|Integer|IncrementInt (Variables|Default|GetInputsDetected)))

(event Custom|SpawnCharacter
  (params (PlayerController :type Player%20Controller%20Object%20Reference) (Team%20Assignment :type ETeam%20Enum :default "NewEnumerator0") (CharacterColor :type Texture%202D%20Object%20Reference))
  (bind _returnvalue (Pawn|GetControlledPawn PlayerController))
  (bind _allplayerstartarray (Variables|Default|GetAllPlayerStartArray))
  (bind _playerstartsteam (CallFunction|FilterPlayerStarts _allplayerstartarray Team%20Assignment))
  (bind _returnvalue_2 (Utilities|Array|Length _playerstartsteam))
  (bind _returnvalue_3 (Math|Random|RandomInteger _returnvalue_2))
  (bind _output (Utilities|Array|Get(acopy) _playerstartsteam _returnvalue_3))
  (bind _returnvalue_4 (Transformation|GetActorTransform _output))
  (Utilities|IsValid _returnvalue
    (:Is%20Valid
      (Actor|DestroyActor _returnvalue)
      (bind _returnvalue_5 (Game|SpawnActorfromClass "/Game/RaidersMain/Blueprints/BP_RaiderMainPlayer.BP_RaiderMainPlayer_C" (Math|Transform|MakeTransform (.location _returnvalue_4) "0,-45.000000, 0" (.scale _returnvalue_4)) "AdjustIfPossibleButAlwaysSpawn" 0 0))
      (Pawn|Possess PlayerController _returnvalue_5)
      (Utilities|Array|AddUnique (Variables|Default|GetPlayers) _returnvalue_5)
      ;[1 1 1] Assign Team
      (Default|AssignTeam _returnvalue_5 Team%20Assignment)
      ;[1 1 1] Color
      (Default|AssignCharcterColor _returnvalue_5 CharacterColor)
      ;[1 1 1] Assign Camera Follow
      (bind _outactors (Actor|GetAllActorsOfClass "/Game/RaidersMain/Blueprints/BP_CameraFollow.BP_CameraFollow_C"))
      (bind _array_element (Utilities|Array|ForEachLoopwithBreak _outactors :!label _label)
        (:LoopBody
          (if (not (Variables|/Game/RaidersMain/Blueprints/BP_CameraFollow.BP_CameraFollow_C|GetisUsed _array_element))
            (Default|NewPlayerJoin _array_element PlayerController _returnvalue_5)
            (goto _label Break)))))))

(event Custom|DespawnPlayer
  (params (PlayerController :type Player%20Controller%20Object%20Reference))
  (bind _returnvalue (Pawn|GetControlledPawn PlayerController))
  (bind _allplayerstartarray (Variables|Default|GetAllPlayerStartArray))
  (Utilities|IsValid _returnvalue
    (:Is%20Valid
      (Actor|DestroyActor _returnvalue)
      (bind _returnvalue_2 (Game|SpawnActorfromClass "/Game/RaidersMain/Blueprints/InitPawn.InitPawn_C" (Transformation|GetActorTransform (Utilities|Array|Get(acopy) _allplayerstartarray (Math|Random|RandomInteger (Utilities|Array|Length _allplayerstartarray)))) "Undefined" 0 0))
      (Pawn|Possess PlayerController _returnvalue_2))))

(event Custom|SpawnPlayers)

(event Custom|RespawnPlayer)

(event EventBeginPlay
  (bind _returnvalue (Class|GameplayStatics|GetPlayerControllerfromID))
  (bind _asraiders_game_instace (Utilities|Casting|CastToRaidersGameInstace (Game|GetGameInstance)))
  (bind _output_get (Variables|Default|Setis1VS1 (Variables|/Game/RaidersMain/Blueprints/RaidersGameInstace.RaidersGameInstace_C|Getstate_is1vs1 _asraiders_game_instace)))
  (if _output_get
    (Variables|Default|SetMaxPlayerCount 1)
    (else
      (Variables|Default|SetMaxPlayerCount 3)))
  (Utilities|FlowControl|Sequence
    (:then_0
      (bind _outactors (Actor|GetAllActorsOfClass "/Game/RaidersMain/Blueprints/BP_RaiderPlayerStart.BP_RaiderPlayerStart_C"))
      (Variables|Default|SetAllPlayerStartArray _outactors)
      ;[1 1 1] Keyboard Player 1
      (Input|EnableInput _returnvalue)
      (Utilities|Array|AddUnique (Variables|Default|GetPlayerControllers) _returnvalue)
      ;[1 1 1] THE REST 3 PLAYERS(PREVIOUS KEYBORD/PAD + 3 PLAYERS PAD
      (for _index (range 1 (Variables|Default|GetMaxPlayerCount))
        (bind _returnvalue_2 (Class|GameplayStatics|CreatePlayer -1))
        (Input|EnableInput _returnvalue_2)
        (Utilities|Array|AddUnique (Variables|Default|GetPlayerControllers) _returnvalue_2)))
    (:then_1
      (if (Variables|Default|Getis1VS1)
        (Utilities|FlowControl|Sequence
          (:then_0
            (CallFunction|SpawnCharacter (Utilities|Array|Get(acopy) (Variables|Default|GetPlayerControllers)) "NewEnumerator0" "/Game/Assets/Raiders/MainCharacter/piel_1_nueva.piel_1_nueva"))
          (:then_1
            (CallFunction|SpawnCharacter (Utilities|Array|Get(acopy) (Variables|Default|GetPlayerControllers) 1) "NewEnumerator1" "/Game/Assets/Raiders/MainCharacter/piel_2_nueva.piel_2_nueva")))
        (else
          (Utilities|FlowControl|Sequence
            (:then_0
              (CallFunction|SpawnCharacter (Utilities|Array|Get(acopy) (Variables|Default|GetPlayerControllers)) "NewEnumerator0" "/Game/Assets/Raiders/MainCharacter/piel_1_nueva.piel_1_nueva"))
            (:then_1
              (CallFunction|SpawnCharacter (Utilities|Array|Get(acopy) (Variables|Default|GetPlayerControllers) 1) "NewEnumerator0" "/Game/Assets/Raiders/MainCharacter/piel_2_nueva.piel_2_nueva"))
            (:then_2
              (CallFunction|SpawnCharacter (Utilities|Array|Get(acopy) (Variables|Default|GetPlayerControllers) 2) "NewEnumerator1" "/Game/Assets/Raiders/MainCharacter/piel_3.piel_3"))
            (:then_3
              (CallFunction|SpawnCharacter (Utilities|Array|Get(acopy) (Variables|Default|GetPlayerControllers) 3) "NewEnumerator1" "/Game/Assets/Raiders/MainCharacter/piel_4_nueva.piel_4_nueva"))))))))

(fn ConstructionScript)

(fn FilterPlayerStarts
  (params (AllStarts :type Array%20of%20BP%20Raider%20Player%20Start%20Object%20References) (TeamFilter :type ETeam%20Enum :default "NewEnumerator0"))
  (for _array_element AllStarts
    (if (Utilities|Enum|Equal(Enum) TeamFilter (Variables|/Game/RaidersMain/Blueprints/BP_RaiderPlayerStart.BP_RaiderPlayerStart_C|GetTeamStart _array_element))
      (Utilities|Array|Add (LocalVariables|GettempPlayerTeam) _array_element)))
  (return (LocalVariables|GettempPlayerTeam)))